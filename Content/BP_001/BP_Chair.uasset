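; BP_Chair is a player-controlled pawn that moves with Enhanced Input and appears to be a practice Blueprint.
; BeginPlay adds the IMC_DIPInput mapping context, and the move action sets MoveDir from its 2D value.
; Tick applies velocity times delta time to the location without sweep, so movement ignores collision.
; Jump only prints press and release messages, while the AddNumber test and an older movement snippet never run.
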(event `self.ReceiveBeginPlay`
  ;[1 1 1] Input 초기 설정하기
  (bind _asplayer_controller (cast `PlayerController` (`self.GetController`)))
  (`/Engine/EditorBlueprintResources/StandardMacros.IsValid` _asplayer_controller
    (:`Is Valid`
      (`EnhancedInputSubsystemInterface.AddMappingContext` (pcsubsystem `EnhancedInputLocalPlayerSubsystem` _asplayer_controller) "/Game/Input/IMC_DIPInput.IMC_DIPInput" 0 (struct)))))

(event `self.ReceiveTick`
  (params (DeltaSeconds :type "Float (single-precision)"))
  ;[1 1 1] P=P0+vt
  (`self.K2_SetActorLocation` (+ (`self.K2_GetActorLocation`) (* (* (`self.MoveDir`) (`self.MoveSpeed`)) DeltaSeconds))))

(event `EnhancedInput|/Game/Input/IA_Jump_DIP`
  (params (ActionValue :type Boolean) (ElapsedSeconds :type "Float (double-precision)") (TriggeredSeconds :type "Float (double-precision)") (InputAction :type "InputAction Object Reference" :default "/Game/Input/IA_Jump_DIP.IA_Jump_DIP"))
  ;[1 1 1] Input 이벤트 설정하기
  (:`Started`
    (`KismetSystemLibrary.PrintString` "Press Space Key!" true true (struct :`R` 1.0 :`G` 1.0 :`A` 1.0) 3.0))
  (:`Completed`
    (`KismetSystemLibrary.PrintString` "Release Space Key!" true true (struct :`R` 1.0 :`A` 1.0) 3.0)))

(event `EnhancedInput|/Game/Input/IA_Move_DIP`
  (params (ActionValue :type "Vector2D Structure") (ElapsedSeconds :type "Float (double-precision)") (TriggeredSeconds :type "Float (double-precision)") (InputAction :type "InputAction Object Reference" :default "/Game/Input/IA_Move_DIP.IA_Move_DIP"))
  ;[1 1 1] Input 이벤트 설정하기
  (:`Triggered`
    (set `self.MoveDir` (`KismetMathLibrary.MakeVector` ActionValue_X ActionValue_Y)))
  (:`Completed`
    (set `self.MoveDir` (`KismetMathLibrary.MakeVector` ActionValue_X ActionValue_Y))))

(fn `AddNumber`
  (params (Num1 :type Integer) (Num2 :type Integer))
  (returns (Result :type Integer))
  (return (+ Num1 Num2)))

(fn `UserConstructionScript`)