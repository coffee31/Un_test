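; Player character Blueprint for a shooter, with Enhanced Input movement, jump, crouch, zoom, rifle fire and grenade throw.
; BeginPlay adds the mapping context and main UI widget; input events store move and rotation values that Tick applies alongside jump/crouch flags and FOV lerp.
; Fire line-traces from the gun muzzle to damage Enemy actors, while Throw launches a physics grenade by impulse.
; The Dash action crouches, and several effect and scoring chains are disconnected.
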(event `self.ReceiveTick`
  (params (DeltaSeconds :type "Float (single-precision)"))
  (bind (_movedir_x _movedir_y) (`KismetMathLibrary.BreakVector` (`self.MoveDir`)))
  (bind (_rotateaxis_roll _rotateaxis_pitch _rotateaxis_yaw) (`KismetMathLibrary.BreakRotator` (`self.RotateAxis`)))
  (bind _springarm (`self.SpringArm`))
  (bind _pc (`self.PC`))
  (bind _returnvalue (`Controller.GetControlRotation` _pc))
  (bind (_returnvalue_roll _returnvalue_pitch _returnvalue_yaw) (`KismetMathLibrary.BreakRotator` (`SceneComponent.K2_GetComponentRotation` _springarm)))
  (`|ExecutionSequence`
    (:`then_0`
      ;[1 1 1] 이동
      (`/Engine/EditorBlueprintResources/StandardMacros.IsValid` _pc
        (:`Is Valid`
          (`self.AddMovementInput` (+ (* (`KismetMathLibrary.GetForwardVector` _returnvalue) _movedir_x) (* (`KismetMathLibrary.GetRightVector` _returnvalue) _movedir_y))))))
    (:`then_1`
      ;[1 1 1] 회전
      (`self.AddControllerYawInput` _rotateaxis_yaw)
      (`SceneComponent.K2_SetWorldRotation` _springarm (`KismetMathLibrary.MakeRotator` _returnvalue_roll (+ _returnvalue_pitch _rotateaxis_pitch) _returnvalue_yaw) false false))
    (:`then_2`
      ;[1 1 1] 착지
      (if (`NavMovementComponent.IsFalling` (`self.CharacterMovement`))
        (set `self.Is_Jump` true)
        (else
          (set `self.Is_Jump` false))))
    (:`then_3`
      (if (`NavMovementComponent.IsCrouching` (`self.CharacterMovement`))
        (set `self.Is_Crouch` true)
        (else
          (set `self.Is_Crouch` false))))
    (:`then_4`
      (`self.CameraZoomINOUT` (* DeltaSeconds 5.0)))))

(event `self.ReceiveBeginPlay`
  (bind _asplayer_controller (cast `PlayerController` (`self.GetController`)))
  (set `self.PC` _asplayer_controller)
  (`EnhancedInputSubsystemInterface.AddMappingContext` (pcsubsystem `EnhancedInputLocalPlayerSubsystem` _asplayer_controller) "/Game/Input/IMC_DIPInput.IMC_DIPInput" 0 (struct))
  (bind _returnvalue (`|CreateWidget` "/Game/UI/WBP_MainUI.WBP_MainUI_C"))
  (bind _output_get (set `self.Main_UI_Inst` _returnvalue))
  (`UserWidget.AddToViewport` _output_get 0))

(event `EnhancedInput|/Game/Input/IA_Jump_DIP`
  (params (ActionValue :type Boolean) (ElapsedSeconds :type "Float (double-precision)") (TriggeredSeconds :type "Float (double-precision)") (InputAction :type "InputAction Object Reference" :default "/Game/Input/IA_Jump_DIP.IA_Jump_DIP"))
  ;[1 1 1] Input 이벤트 설정하기
  (:`Started`
    (if (not (`NavMovementComponent.IsFalling` (`self.CharacterMovement`)))
      (`self.Jump`)
      (set `self.Is_Jump` true)))
  (:`Completed`
    (`self.StopJumping`)))

(event `EnhancedInput|/Game/Input/IA_Dash_DIP`
  (params (ActionValue :type Boolean) (ElapsedSeconds :type "Float (double-precision)") (TriggeredSeconds :type "Float (double-precision)") (InputAction :type "InputAction Object Reference" :default "/Game/Input/IA_Dash_DIP.IA_Dash_DIP"))
  ;[1 1 1] Input 이벤트 설정하기
  (:`Triggered`
    (`self.Crouch`)
    (set `self.Is_Crouch` true))
  (:`Completed`
    (`self.UnCrouch`)))

(event `EnhancedInput|/Game/Input/IA_ZOOM_DIP`
  (params (ActionValue :type Boolean) (ElapsedSeconds :type "Float (double-precision)") (TriggeredSeconds :type "Float (double-precision)") (InputAction :type "InputAction Object Reference" :default "/Game/Input/IA_ZOOM_DIP.IA_ZOOM_DIP"))
  (bind _springarm (`self.SpringArm`))
  (:`Started`
    (set `SpringArmComponent.TargetArmLength` -100.0 _springarm)
    (set `self.Fov` 45.0))
  (:`Completed`
    (set `SpringArmComponent.TargetArmLength` 500.0 _springarm)
    (set `self.Fov` 90.0)))

(event `EnhancedInput|/Game/Input/IA_Move_DIP`
  (params (ActionValue :type "Vector2D Structure") (ElapsedSeconds :type "Float (double-precision)") (TriggeredSeconds :type "Float (double-precision)") (InputAction :type "InputAction Object Reference" :default "/Game/Input/IA_Move_DIP.IA_Move_DIP"))
  ;[1 1 1] Input 이벤트 설정하기
  (:`Triggered`
    (set `self.MoveDir` (`KismetMathLibrary.MakeVector` ActionValue_X ActionValue_Y)))
  (:`Completed`
    (set `self.MoveDir` (`KismetMathLibrary.MakeVector` ActionValue_X ActionValue_Y))))

(event `EnhancedInput|/Game/Input/IA_Roate_DIP`
  (params (ActionValue :type "Vector2D Structure") (ElapsedSeconds :type "Float (double-precision)") (TriggeredSeconds :type "Float (double-precision)") (InputAction :type "InputAction Object Reference" :default "/Game/Input/IA_Roate_DIP.IA_Roate_DIP"))
  ;[1 1 1] Input 이벤트 설정하기
  (:`Triggered`
    (set `self.RotateAxis` (`KismetMathLibrary.MakeRotator` 0.0 ActionValue_Y ActionValue_X)))
  (:`Completed`
    (set `self.RotateAxis` (`KismetMathLibrary.MakeRotator` 0.0 ActionValue_Y ActionValue_X))))

(event `EnhancedInput|/Game/Input/IA_Fire_DIP`
  (params (ActionValue :type Boolean) (ElapsedSeconds :type "Float (double-precision)") (TriggeredSeconds :type "Float (double-precision)") (InputAction :type "InputAction Object Reference" :default "/Game/Input/IA_Fire_DIP.IA_Fire_DIP"))
  (bind _gunmesh (`self.GunMesh`))
  (bind _returnvalue (`SceneComponent.GetSocketLocation` _gunmesh "Muzzle"))
  (:`Started`
    (bind _outhit (`KismetSystemLibrary.LineTraceSingle` :`Start` _returnvalue :`End` (+ _returnvalue (* (`SceneComponent.GetRightVector` _gunmesh) 1000.0)) :`TraceChannel` "TraceTypeQuery1" :`DrawDebugType` "ForDuration"))
    (bind _asenemy (cast `Enemy` (`.HitActor` (`GameplayStatics.BreakHitResult` _outhit))))
    (`Enemy.OnDamager` _asenemy (`self.RiflePower`))
    (bind _returnvalue_2 (`Enemy.GetCurrentHP` _asenemy))
    (if (== _returnvalue_2 0)
      _)))

(event `EnhancedInput|/Game/Input/IA_Throw_DIP`
  (params (ActionValue :type Boolean) (ElapsedSeconds :type "Float (double-precision)") (TriggeredSeconds :type "Float (double-precision)") (InputAction :type "InputAction Object Reference" :default "/Game/Input/IA_Throw_DIP.IA_Throw_DIP"))
  (:`Completed`
    (bind _returnvalue (`|SpawnActorFromClass` "/Game/BP_001/BP_Granade.BP_Granade_C" (`SceneComponent.GetSocketTransform` (`self.GunMesh`) "Muzzle" "RTS_World") "Undefined" "MultiplyWithRoot" null null))
    (bind _asgranade_actor (cast `GranadeActor` _returnvalue))
    (`|ExecutionSequence`
      (:`then_0`
        (bind _spherecollision (`GranadeActor.SphereCollision` _asgranade_actor))
        (`PrimitiveComponent.SetCollisionEnabled` _spherecollision "QueryAndPhysics")
        (`PrimitiveComponent.SetSimulatePhysics` _spherecollision true)
        (`PrimitiveComponent.SetEnableGravity` _spherecollision true))
      (:`then_1`
        (bind _rootcomponent (`Actor.RootComponent` _asgranade_actor))
        (`PrimitiveComponent.AddImpulse` _spherecollision (* (`KismetMathLibrary.Normal` (+ (`SceneComponent.GetForwardVector` _rootcomponent) (`SceneComponent.GetUpVector` _rootcomponent))) (`self.ThrowPower`)) "None" false))
      (:`then_2`
        (`self.PlayAnimMontage` "/Game/FirstPersonArms/Animations/FP_Rifle_Shoot_Montage.FP_Rifle_Shoot_Montage")))))

(fn `CameraZoomINOUT`
  (params (Rate :type "Float (double-precision)"))
  (bind _camera (`self.Camera`))
  (`CameraComponent.SetFieldOfView` _camera (`KismetMathLibrary.Lerp` (`CameraComponent.FieldOfView` _camera) (`self.Fov`) Rate))
  (return))

(fn `UserConstructionScript`)